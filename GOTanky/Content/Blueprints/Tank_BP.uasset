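; Player-controllable tank Blueprint that wires input to its track, aiming and camera components.
; On begin play it hands the turret and barrel to TankAiming and both tracks to TankMovement, and track hit events call each track's OnHit.
; Driving works either through per-track throttle axes or move and turn intents sent to TankMovement.
; Aim axes rotate the azimuth gimbal and spring arm, while Fire triggers TankAiming.
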(event OnComponentHit(RightTrack)
  (params (HitComponent :type Primitive%20Component%20Object%20Reference) (OtherActor :type Actor%20Object%20Reference) (OtherComp :type Primitive%20Component%20Object%20Reference) (NormalImpulse :type Vector :default "0, 0, 0") (Hit :type Hit%20Result%20Structure%20%28by%20ref%29))
  (Class|TankTrack|OnHit (Variables|Default|GetRight%20Track)))

(event OnComponentHit(LeftTrack)
  (params (HitComponent :type Primitive%20Component%20Object%20Reference) (OtherActor :type Actor%20Object%20Reference) (OtherComp :type Primitive%20Component%20Object%20Reference) (NormalImpulse :type Vector :default "0, 0, 0") (Hit :type Hit%20Result%20Structure%20%28by%20ref%29))
  (Class|TankTrack|OnHit (Variables|Default|GetLeft%20Track)))

(event EventBeginPlay
  (Class|TankAimingComponent|Initialise (Variables|Default|GetTankAiming) (Variables|Default|GetTurret) (Variables|Default|GetBarrel))
  (Class|TankMovementComponent|Initialise (Variables|Default|GetTankMovement) (Variables|Default|GetRight%20Track) (Variables|Default|GetLeft%20Track)))

(event Input|ActionEvents|InputActionFire
  (params (Key :type Key%20Structure :default "AnyKey"))
  ;[1 1 1] Firing
  (:Pressed
    (Class|TankAimingComponent|Fire (Variables|Default|GetTankAiming))))

(event Input|AxisEvents|InputAxisAimAzimuth
  (params (AxisValue :type Float%20%28single-precision%29))
  ;[1 1 1] AimAzimuth
  (Transformation|AddLocalRotation (Variables|Default|GetAzimuth%20Gimbal) (Math|Rotator|MakeRotator 0.0 0.0 AxisValue) false false))

(event Input|AxisEvents|InputAxisTurnLeft
  (params (AxisValue :type Float%20%28single-precision%29))
  ;[1 1 1] Movement Input Binding
  (Class|TankMovementComponent|IntendTurnLeft (Variables|Default|GetTankMovement) AxisValue))

(event Input|AxisEvents|InputAxisAimElevation
  (params (AxisValue :type Float%20%28single-precision%29))
  ;[1 1 1] AimElevation
  (Transformation|AddLocalRotation (Variables|Default|GetSpringArm) (Math|Rotator|MakeRotator 0.0 AxisValue 0.0) false false))

(event Input|AxisEvents|InputAxisTurnRight
  (params (AxisValue :type Float%20%28single-precision%29))
  ;[1 1 1] Movement Input Binding
  (Class|TankMovementComponent|IntendTurnRight (Variables|Default|GetTankMovement) AxisValue))

(event Input|AxisEvents|InputAxisMoveForward
  (params (AxisValue :type Float%20%28single-precision%29))
  ;[1 1 1] Movement Input Binding
  (Class|TankMovementComponent|IntendMoveForward (Variables|Default|GetTankMovement) AxisValue))

(event Input|AxisEvents|InputAxisMoveBackwards
  (params (AxisValue :type Float%20%28single-precision%29))
  ;[1 1 1] Movement Input Binding
  (Class|TankMovementComponent|IntendMoveBackwards (Variables|Default|GetTankMovement) AxisValue))

(event Input|AxisEvents|InputAxisLeftTrackThrottle
  (params (AxisValue :type Float%20%28single-precision%29))
  ;[1 1 1] Movement Input Binding
  (Class|TankTrack|SetThrottle (Variables|Default|GetLeft%20Track) AxisValue))

(event Input|AxisEvents|InputAxisRightTrackThrottle
  (params (AxisValue :type Float%20%28single-precision%29))
  ;[1 1 1] Movement Input Binding
  (Class|TankTrack|SetThrottle (Variables|Default|GetRight%20Track) AxisValue))

(fn ConstructionScript)